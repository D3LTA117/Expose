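; Stabilité2 is an overlap-reactive Blueprint that blanks a group of seven French and Japanese-titled text elements, apparently on Japanese work culture and management.
; Both begin and end overlap set every element, such as ShûshinKoyô, NenkôJoretsu and GestionAméricaine, to an empty string.
; The events do not check which actor overlaps, and the construction script is empty.
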(event `self.ReceiveActorBeginOverlap`
  (params (OtherActor :type "Actor Object Reference"))
  (`TextRenderComponent.K2_SetText` (`self.1994`) "")
  (`TextRenderComponent.K2_SetText` (`self.Structure`) "")
  (`TextRenderComponent.K2_SetText` (`self.Shûshin Koyô`) "")
  (`TextRenderComponent.K2_SetText` (`self.Domaines`) "")
  (`TextRenderComponent.K2_SetText` (`self.EthiqueTravail`) "")
  (`TextRenderComponent.K2_SetText` (`self.Nenkô Joretsu`) "")
  (`TextRenderComponent.K2_SetText` (`self.GestionAméricaine`) ""))

(event `self.ReceiveActorEndOverlap`
  (params (OtherActor :type "Actor Object Reference"))
  (`TextRenderComponent.K2_SetText` (`self.1994`) "")
  (`TextRenderComponent.K2_SetText` (`self.Structure`) "")
  (`TextRenderComponent.K2_SetText` (`self.Shûshin Koyô`) "")
  (`TextRenderComponent.K2_SetText` (`self.Domaines`) "")
  (`TextRenderComponent.K2_SetText` (`self.EthiqueTravail`) "")
  (`TextRenderComponent.K2_SetText` (`self.Nenkô Joretsu`) "")
  (`TextRenderComponent.K2_SetText` (`self.GestionAméricaine`) ""))

(fn `UserConstructionScript`)