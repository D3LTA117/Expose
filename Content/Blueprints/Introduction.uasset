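; Introduction Blueprint that reacts to actor overlaps by writing to a set of text objects with French titles and years, such as Intronisation, Funérailles and 1989.
; Begin overlap sets all of them, including Intro, to the literal "Entered Volume".
; End overlap writes the same string to every one except Intro, so leaving neither clears nor restores the text.
; The construction script is empty.
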(event `self.ReceiveActorBeginOverlap`
  (params (OtherActor :type "Actor Object Reference"))
  (`TextRenderComponent.K2_SetText` (`self.Ouvrage`) "Entered Volume")
  (`TextRenderComponent.K2_SetText` (`self.1992`) "Entered Volume")
  (`TextRenderComponent.K2_SetText` (`self.1990`) "Entered Volume")
  (`TextRenderComponent.K2_SetText` (`self.PNB`) "Entered Volume")
  (`TextRenderComponent.K2_SetText` (`self.Intronisation`) "Entered Volume")
  (`TextRenderComponent.K2_SetText` (`self.1989`) "Entered Volume")
  (`TextRenderComponent.K2_SetText` (`self.Funérailles`) "Entered Volume")
  (`TextRenderComponent.K2_SetText` (`self.Intro`) "Entered Volume"))

(event `self.ReceiveActorEndOverlap`
  (params (OtherActor :type "Actor Object Reference"))
  (`TextRenderComponent.K2_SetText` (`self.Ouvrage`) "Entered Volume")
  (`TextRenderComponent.K2_SetText` (`self.1992`) "Entered Volume")
  (`TextRenderComponent.K2_SetText` (`self.1990`) "Entered Volume")
  (`TextRenderComponent.K2_SetText` (`self.PNB`) "Entered Volume")
  (`TextRenderComponent.K2_SetText` (`self.Intronisation`) "Entered Volume")
  (`TextRenderComponent.K2_SetText` (`self.1989`) "Entered Volume")
  (`TextRenderComponent.K2_SetText` (`self.Funérailles`) "Entered Volume"))

(fn `UserConstructionScript`)